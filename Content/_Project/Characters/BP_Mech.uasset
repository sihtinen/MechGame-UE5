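; Player-controllable modular mech pawn that builds its legs, body, arms and head meshes and anim blueprints from loadout equipment assets.
; Enhanced Input drives curve-scaled stick look and mouse look, and stores move and boost input.
; On player possession it spawns HUD and targeting-area widgets, feeds reticle location between them, and culls MechTargeting options outside that area.
; It keeps its physics capsule awake and includes debug arrows and frame-rate keys.
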(event Input|EnhancedActionEvents|EnhancedInputActionIA_MouseLook
  (params (ActionValue :type Vector%202D%20Structure) (ElapsedSeconds :type Float%20%28double-precision%29) (TriggeredSeconds :type Float%20%28double-precision%29) (InputAction :type Input%20Action%20Object%20Reference :default "/Game/_Project/Input/IA_MouseLook.IA_MouseLook"))
  ;[1 1 1] Mouse Look Input
  (Pawn|Input|AddControllerYawInput (.x ActionValue))
  (Pawn|Input|AddControllerPitchInput (* (.y ActionValue) -1.0)))

(event Input|EnhancedActionEvents|EnhancedInputActionIA_Move
  (params (ActionValue :type Vector%202D%20Structure) (ElapsedSeconds :type Float%20%28double-precision%29) (TriggeredSeconds :type Float%20%28double-precision%29) (InputAction :type Input%20Action%20Object%20Reference :default "/Game/_Project/Input/IA_Move.IA_Move"))
  ;[1 1 1] Move Input
  (:Triggered
    (Variables|Default|SetMoveInput ActionValue))
  (:Canceled
    (Variables|Default|SetMoveInput (Utilities|Struct|MakeVector2f 0.0 0.0) :!label _label))
  (:Completed
    (goto _label)))

(event Input|EnhancedActionEvents|EnhancedInputActionIA_Look
  (params (ActionValue :type Vector%202D%20Structure) (ElapsedSeconds :type Float%20%28double-precision%29) (TriggeredSeconds :type Float%20%28double-precision%29) (InputAction :type Input%20Action%20Object%20Reference :default "/Game/_Project/Input/IA_Look.IA_Look"))
  (bind _returnvalue (Utilities|Time|GetWorldDeltaSeconds))
  (bind _returnvalue_2 (Math|Vector2D|MakeVector2D (.x ActionValue) (.y ActionValue)))
  (bind _lookresponsecurve (Variables|Default|GetLookResponseCurve))
  (bind _returnvalue_3 (Math|Vector2D|Vector2DLength _returnvalue_2))
  (bind _returnvalue_4 (Math|Curves|GetFloatValue _lookresponsecurve _returnvalue_3))
  ;[1 1 1] Controller Look Input
  (Pawn|Input|AddControllerYawInput (* (* (.x ActionValue) _returnvalue_4) _returnvalue (Variables|Default|GetLookSensitivityYaw)))
  (Pawn|Input|AddControllerPitchInput (* (* (.y ActionValue) _returnvalue_4) _returnvalue (Variables|Default|GetLookSensitivityPitch))))

(event Input|EnhancedActionEvents|EnhancedInputActionIA_ShoulderLeft
  (params (ActionValue :type Boolean) (ElapsedSeconds :type Float%20%28double-precision%29) (TriggeredSeconds :type Float%20%28double-precision%29) (InputAction :type Input%20Action%20Object%20Reference :default "/Game/_Project/Input/IA_ShoulderLeft.IA_ShoulderLeft"))
  ;[1 1 1] Left Shoulder Input
  (:Started
    (Variables|Default|SetbBoostInputActive true))
  (:Canceled
    (Variables|Default|SetbBoostInputActive false :!label _label))
  (:Completed
    (goto _label)))

(event EventBeginPlay
  ;[1 1 1] Begin Play
  (|BeginPlayGraph))

(event EventOnLoadoutAssetsLoadedtoMemory
  ;[1 1 1] On Loadout Assets Load Completed
  (CallFunction|UpdateSkinnedMeshes))

(event EventTick
  (params (DeltaSeconds :type Float%20%28single-precision%29))
  ;[1 1 1] Event Tick
  (CallFunction|DrawDirectionArrow)
  (Variables|/Game/_Project/Widgets/WBP_TargetingArea.WBP_TargetingArea_C|SetReticleTargetLocation (Variables|Default|GetTargetingAreaWidget) (Default|GetReticleLocation (Variables|Default|GetHUDWidget))))

(event EventPossessed
  (params (NewController :type Controller%20Object%20Reference))
  ;[1 1 1] On Possessed Event
  (CallFunction|SpawnTargetingAreaWidgetActor NewController)
  (CallFunction|SpawnHUDWidget NewController))

(event Input|KeyboardEvents|DebugKey5
  (params (Key :type Key%20Structure) (ActionValue :type Input%20Action%20Value%20Structure))
  (:Pressed
    (Class|Mech|SetFixedFrameRate 30)))

(event Input|KeyboardEvents|DebugKey6
  (params (Key :type Key%20Structure) (ActionValue :type Input%20Action%20Value%20Structure))
  (:Pressed
    (Class|Mech|SetFixedFrameRate 60)))

(event Input|KeyboardEvents|DebugKey7
  (params (Key :type Key%20Structure) (ActionValue :type Input%20Action%20Value%20Structure))
  (:Pressed
    (Class|Mech|SetFixedFrameRate 144)))

(fn ConstructionScript)

(fn MapPlayerInput
  (bind _asplayer_controller (Utilities|Casting|CastToPlayerController (Pawn|GetController)))
  (Utilities|IsValid (PlayerController|LocalPlayerSubsystems|GetEnhancedInputLocalPlayerSubsystem _asplayer_controller)
    (:Is%20Valid
      (Input|AddMappingContext (PlayerController|LocalPlayerSubsystems|GetEnhancedInputLocalPlayerSubsystem _asplayer_controller) "/Game/_Project/Input/IMC_Default.IMC_Default" 0 "(bIgnoreAllPressedKeysUntilRelease=True,bForceImmediately=False,bNotifyUserSettings=False)"))))

(fn UpdateSkinnedMeshes
  (bind _loadoutasset (Variables|Default|GetLoadoutAsset))
  (bind _loadoutasset_2 (Variables|Default|GetLoadoutAsset))
  (bind _slots (Variables|/Script/MechGame.MechLoadoutAsset|GetSlots _loadoutasset))
  (Utilities|IsValid _loadoutasset_2
    (:Is%20Valid
      (bind _success (CallFunction|SetSkinnedMeshfromEquipmentAsset (.Value (Utilities|Map|Find (Variables|/Script/MechGame.MechLoadoutAsset|GetSlots _loadoutasset_2) "Legs")) (Variables|Default|GetLegs)))
      (if _success
        (Utilities|FlowControl|Sequence
          (:then_0
            (CallFunction|SetSkinnedMeshfromEquipmentAsset (.Value (Utilities|Map|Find _slots "Body")) (Variables|Default|GetBody)))
          (:then_1
            (CallFunction|SetSkinnedMeshfromEquipmentAsset (.Value (Utilities|Map|Find _slots "Arms")) (Variables|Default|GetArms)))
          (:then_2
            (CallFunction|SetSkinnedMeshfromEquipmentAsset (.Value (Utilities|Map|Find _slots "Head")) (Variables|Default|GetHead))))))))

(fn SetSkinnedMeshfromEquipmentAsset
  (params (EquipmentAsset :type Mech%20Equipment%20Asset%20Object%20Reference) (SkeletalMeshComponent :type Skeletal%20Mesh%20Component%20Object%20Reference))
  (bind _mesh (Variables|/Script/MechGame.MechEquipmentAsset|GetMesh EquipmentAsset))
  (Utilities|IsValid EquipmentAsset
    (:Is%20Valid
      (if (and (Utilities|IsValidSoftObjectReference _mesh) true)
        (Components|SkinnedMesh|SetSkinnedAssetandUpdate SkeletalMeshComponent (Utilities|ResolveSoftReference _mesh) true)
        (Class|Mech|SetAnimationBlueprint SkeletalMeshComponent (Variables|/Script/MechGame.MechEquipmentAsset|GetAnimBlueprint EquipmentAsset))
        (return true)
        (else
          _)))
    (:Is%20Not%20Valid
      _))
  (return false))

(fn SpawnTargetingAreaWidgetActor
  (params (PawnController :type Controller%20Object%20Reference))
  (if (Class|Controller|IsPlayerController PawnController)
    (bind _returnvalue (UserInterface|CreateWidget "/Game/_Project/Widgets/WBP_TargetingArea.WBP_TargetingArea_C" (Game|GetPlayerController 0) "/Game/_Project/Widgets/DA_HUDSettings.DA_HUDSettings"))
    (bind _output_get (Variables|Default|SetTargetingAreaWidget _returnvalue))
    (Default|BindtoSource _output_get self)
    (UserInterface|Viewport|AddtoViewport _output_get 0)))

(fn SpawnHUDWidget
  (params (ControllerPawn :type Controller%20Object%20Reference))
  (if (Class|Controller|IsPlayerController ControllerPawn)
    (bind _returnvalue (UserInterface|CreateWidget "/Game/_Project/Widgets/WBP_HUD.WBP_HUD_C" (Game|GetPlayerController 0) "/Game/_Project/Widgets/DA_HUDSettings.DA_HUDSettings"))
    (bind _output_get (Variables|Default|SetHUDWidget _returnvalue))
    (UserInterface|Viewport|AddtoViewport _output_get 0)))

(fn DrawDirectionArrow
  (bind _returnvalue (Class|Mech|GetPivotWorldLocation false))
  (Rendering|Debug|DrawDebugArrow _returnvalue (+ _returnvalue (* (Transformation|GetActorForwardVector) "100.000000,100.000000,100.000000")) 0.0 "(R=0.000000,G=0.599663,B=1.000000,A=1.000000)" 0.0 1.0))

(fn OnValidTargetingOptionsCollected
  (bind _mechtargeting (Variables|Default|GetMechTargeting))
  (bind _validtargetingoptions (Variables|/Script/MechGame.MechTargetingComponent|GetValidTargetingOptions _mechtargeting))
  (if (Class|Controller|IsPlayerController (Pawn|GetController))
    (bind (_arrayindex _arrayelement) (Utilities|Array|ReverseforEachLoop _validtargetingoptions)
      (:LoopBody
        (bind _resultvalue (Default|IsLocationInsideTargetingArea (Variables|Default|GetTargetingAreaWidget) (Game|GetPlayerController 0) (Transformation|GetActorLocation (Components|GetOwner (.contexttargetcomponent _arrayelement)))))
        (if _resultvalue
          (Rendering|Debug|DrawDebugArrow (Transformation|GetActorLocation) (Transformation|GetActorLocation (Components|GetOwner (.contexttargetcomponent _arrayelement))) 0.0 "(R=0.022470,G=1.000000,B=0.000000,A=1.000000)" 0.0 1.0)
          (else
            (Utilities|Array|RemoveIndex _validtargetingoptions _arrayindex)))))))

(event Custom|OnValidTargetingOptionsCollected_Event
  (CallFunction|OnValidTargetingOptionsCollected))

(event Custom|OnCapsuleSleepEvent
  (params (SleepingComponent :type Primitive%20Component%20Object%20Reference) (BoneName :type Name))
  (Class|PrimitiveComponent|WakeRigidBody SleepingComponent "None"))

(fn GetState
  (return (Transformation|GetBoneTransform (Variables|Default|GetHead) "head" "RTS_World") (Transformation|GetWorldTransform (Variables|Default|GetCamera))))